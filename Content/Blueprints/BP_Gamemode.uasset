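; Game mode Blueprint that runs a countdown game timer and loads EndMap once it runs out.
; On BeginPlay it creates the WBP_GameMenu HUD, sets game-only input with a hidden cursor, and shows the starting timer and score.
; Tick calls UpdateTimer, whose one-second Delay throttles the decrement to about once per second and refreshes the HUD.
; At zero or below, another one-second Delay precedes the level change.
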(event `self.ReceiveBeginPlay`
  (`KismetSystemLibrary.PrintString` (`self.Starting String`))
  (`self.SpawnGameMenu`)
  (`/Game/Blueprints/GUI/GameMenu/WBP_GameMenu.SetTimer` (`self.MenuRef`) (`self.GameTimer'`))
  (`/Game/Blueprints/GUI/GameMenu/WBP_GameMenu.SetScore` (`self.MenuRef`) (`self.Score`)))

(event `self.ReceiveTick`
  (params (DeltaSeconds :type "Float (single-precision)"))
  (`self.UpdateTimer`)
  (if (<= (`self.GameTimer'`) 0)
    (`KismetSystemLibrary.Delay` 1.0)
    (`GameplayStatics.OpenLevelBySoftObjectPtr` "/Game/Map/EndMap.EndMap")))

(fn `SpawnGameMenu`
  (bind _returnvalue (`GameplayStatics.GetPlayerController` 0))
  (bind _returnvalue_2 (`|CreateWidget` "/Game/Blueprints/GUI/GameMenu/WBP_GameMenu.WBP_GameMenu_C"))
  (bind _output_get (set `self.MenuRef` _returnvalue_2))
  (`UserWidget.AddToViewport` _output_get 0)
  (`WidgetBlueprintLibrary.SetInputMode_GameOnly` _returnvalue)
  (set `PlayerController.bShowMouseCursor` false _returnvalue))

(fn `UserConstructionScript`)